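; Sword actor that gets picked up into its owner's sword array and strikes Snake02 enemies.
; Timelines drive pickup spin, socket-chained attachment, material fade and moves to target slots, where a looping timer line-traces for damage.
; Capsule hits on a snake's head or body remove it from YaQi's array, reduce snake HP and send it flying before destruction.
; Another function drops a weapon with physics; older Snake hit logic is unconnected.
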(event OnComponentBeginOverlap(Capsule)
  (params (OverlappedComponent :type Primitive%20Component%20Object%20Reference) (OtherActor :type Actor%20Object%20Reference) (OtherComp :type Primitive%20Component%20Object%20Reference) (OtherBodyIndex :type Integer) (bFromSweep :type Boolean) (SweepResult :type Hit%20Result%20Structure%20%28by%20ref%29))
  (bind _as_ya_qi (Variables|Default|GetAs%20Ya%20Qi))
  (bind _as_ya_qi_2 (Variables|Default|GetAs%20Ya%20Qi))
  (bind _assnake_02 (Utilities|Casting|CastToSnake02 OtherActor)
    (:then
      (CallFunction|Stop)
      (Utilities|FlowControl|DoOnce false
        (:Completed
          (Utilities|FlowControl|Sequence
            (:then_0
              (Utilities|Array|RemoveItem (Variables|/Game/YaQi/Bp/YaQi.YaQi_C|GetArraySword _as_ya_qi_2) self)
              (Math|Integer|DecrementInt (Variables|/Game/YaQi/Bp/YaQi.YaQi_C|Get每圈数量 _as_ya_qi_2)
                (:%20%20
                  (Collision|SetCollisionEnabled (Variables|Default|GetCapsule) "NoCollision")
                  (Transformation|DetachFromActor "KeepWorld" "KeepWorld" "KeepWorld")
                  (Audio|PlaySoundatLocation "/Game/YaQi/Audios/Hit.Hit" (Transformation|GetActorLocation) "0, 0, 0" 1.0 1.0 0.0 0 0 0 0)
                  (Utilities|Time|SetTimerbyFunctionName 0 "MoveForward" 0.01 true))))
            (:then_1
              (Utilities|FlowControl|Delay 1.0)
              (Actor|DestroyActor))
            (:then_2
              (Default|HeadHit _assnake_02)
              (Effects|SpawnEmitteratLocation "/Game/LoPoPack/Particles/Par_LoPo_Spark_02.Par_LoPo_Spark_02" (Transformation|GetWorldLocation (Variables|Default|GetScene1)) "0, 0, 0" "0.300000,0.300000,0.300000"))
            (:then_3
              (Default|ReduceHp _assnake_02))))))
    (:CastFailed
      (bind _assnake_02_body (Utilities|Casting|CastToSnake02_Body OtherActor))
      (Utilities|FlowControl|DoOnce false
        (:Completed
          (Utilities|FlowControl|Sequence
            (:then_0
              (Utilities|Array|RemoveItem (Variables|/Game/YaQi/Bp/YaQi.YaQi_C|GetArraySword _as_ya_qi) self)
              (Math|Integer|DecrementInt (Variables|/Game/YaQi/Bp/YaQi.YaQi_C|Get每圈数量 _as_ya_qi)
                (:%20%20
                  (Collision|SetCollisionEnabled (Variables|Default|GetCapsule) "NoCollision")
                  (Transformation|DetachFromActor "KeepWorld" "KeepWorld" "KeepWorld")
                  (Audio|PlaySoundatLocation "/Game/YaQi/Audios/Hit.Hit" (Transformation|GetActorLocation) "0, 0, 0" 1.0 1.0 0.0 0 0 0 0)
                  (Utilities|Time|SetTimerbyFunctionName 0 "MoveForward" 0.01 true))))
            (:then_1
              (Utilities|FlowControl|Delay 1.0)
              (Actor|DestroyActor))
            (:then_2
              (Effects|SpawnEmitteratLocation "/Game/LoPoPack/Particles/Par_LoPo_Spark_02.Par_LoPo_Spark_02" (Transformation|GetWorldLocation (Variables|Default|GetScene1)) "0, 0, 0" "0.300000,0.300000,0.300000"))
            (:then_3
              (Default|ReduceHp (.AsSnake%2002 (Utilities|Casting|CastToSnake02 (Actor|GetAttachParentActor _assnake_02_body)))))))))))

(event Custom|出现
  ;[1 1 1] 出现
  ;;[1 1 1] 吸入完成的时候开启碰撞检测
  (Variables|/Script/Engine.PrimitiveComponent|SetbGenerateOverlapEvents (Variables|Default|GetSkeletal) true)
  (Components|Timeline|SetPlayRate (Variables|Default|GetTL_出现) 5.0)
  (bind (_direction _旋转 _newtrack_1) (Timeline|TL_出现 PlayFromStart)
    (:Update
      (Transformation|SetRelativeRotation (Variables|Default|GetArrow) (Math|Rotator|MakeRotator 0.0 0.0 (Math|Float|Lerp 1.8e+02 0.0 _旋转)) false false)
      (Rendering|Material|SetScalarParameterValueonMaterials (Variables|Default|GetSkeletal) "EM" _newtrack_1))
    (:Finished
      (Default|计算特效位置 (.AsBP%20Spawn%20Sword (Utilities|Casting|CastToBP_SpawnSword (Variables|1|Get主人)))))))

(event Custom|被捡
  (params (目标 :type BP%20Spawn%20Sword%20Object%20Reference) (Scene :type Scene%20Component%20Object%20Reference))
  (bind _剑数组 (Variables|/Game/BP/Weapon/Sword/BP_SpawnSword.BP_SpawnSword_C|Get剑数组 目标))
  ;[1 1 1] 被捡
  (Variables|1|Set主人 目标)
  ;;[1 1 1] 被吸入的时候关闭碰撞检测
  (Variables|/Script/Engine.PrimitiveComponent|SetbGenerateOverlapEvents (Variables|Default|GetSkeletal) false)
  (Variables|1|Set初始位置 (Transformation|GetActorLocation))
  (Components|Timeline|SetPlayRate (Variables|Default|GetTL_被捡) 4e+01)
  (bind _newtrack_0 (Timeline|TL_被捡 PlayFromStart)
    (:Update
      (Transformation|SetActorRotation (Math|Rotator|MakeRotator 0.0 0.0 (Math|Float|Lerp 0.0 3.6e+02 _newtrack_0))))
    (:Finished
      (Transformation|AttachComponentToComponent Scene "" "KeepWorld" "KeepRelative" "SnapToTarget" true)
      (Transformation|SetActorLocation (Transformation|GetSocketLocation (Variables|BP_Sword_C|GetSkeletal (Utilities|Array|Get(acopy) _剑数组 (Utilities|Array|LastIndex _剑数组))) "pingjie") false false)
      (Utilities|Array|AddUnique (Variables|/Game/BP/Weapon/Sword/BP_SpawnSword.BP_SpawnSword_C|Get剑数组 目标) self)
      (CallFunction|出现)
      ;;[1 1 1] 调整位置
      (Default|调整位置 目标 false)
      (Default|计算特效位置 (.AsBP%20Spawn%20Sword (Utilities|Casting|CastToBP_SpawnSword (Variables|1|Get主人)))))))

(event Custom|MoveToTarget
  (params (Actor :type BP%20Spawn%20Sword%20Object%20Reference) (Index :type Integer))
  (bind _tarlocarray (Variables|/Game/BP/Weapon/Sword/BP_SpawnSword.BP_SpawnSword_C|GetTarLocArray Actor))
  (bind _output (Utilities|Array|Get(acopy) _tarlocarray Index))
  (bind _returnvalue (Transformation|GetWorldTransform _output))
  ;[1 1 1] MoveToTarget
  (Transformation|DetachFromActor "KeepWorld" "KeepWorld" "KeepWorld")
  (Variables|1|Set初始位置 (Transformation|GetActorLocation))
  (Variables|Default|SetCurrentRotation (Transformation|GetActorRotation))
  (Components|Timeline|SetPlayRate (Variables|Default|GetTL_MoveToTarget) 5.0)
  (bind _newtrack_0 (Timeline|TL_MoveToTarget PlayFromStart)
    (:Update
      (Transformation|SetActorLocation (Math|Vector|Lerp(Vector) (Variables|1|Get初始位置) (.location _returnvalue) _newtrack_0) false false)
      (Transformation|SetActorRotation (Math|Rotator|MakeRotator 0.0 0.0 (Math|Float|Lerp (.yaw (Variables|Default|GetCurrentRotation)) (.Yaw (Math|Rotator|BreakRotator (.rotation _returnvalue))) _newtrack_0))))
    (:Finished
      (Transformation|AttachComponentToComponent _output "None" "KeepWorld" "KeepWorld" "SnapToTarget" true)
      (bind _returnvalue_2 (Utilities|Time|SetTimerbyFunctionName 0 "CheckDamage" 0.01 true))
      (Variables|Default|SetCheckDamageHandle _returnvalue_2))))

(event Custom|Fly
  ;[1 1 1] Comment
  (Transformation|DetachFromActor "KeepWorld" "KeepWorld" "KeepWorld")
  (Utilities|Time|SetTimerbyFunctionName 0 "MoveForward" 0.01 true))

(event Custom|Move
  (params (NewParam :type Arrow%20Component%20Object%20Reference))
  (bind _returnvalue (Transformation|GetWorldTransform NewParam))
  (Variables|Default|SetNewVar (Transformation|GetActorLocation))
  (Variables|Default|SetNewVar_0 (Transformation|GetActorRotation))
  (Components|Timeline|SetPlayRate (Variables|Default|GetTimeline) 4.0)
  (bind _newtrack_0 (Timeline|Timeline PlayFromStart)
    (:Update
      (Transformation|SetActorLocationAndRotation (Math|Vector|Lerp(Vector) (Variables|Default|GetNewVar) (.location _returnvalue) _newtrack_0) (Math|Rotator|Lerp(Rotator) (Variables|Default|GetNewVar_0) (.rotation _returnvalue) _newtrack_0 true)))))

(event Custom|Stop
  (bind _newtrack_0 (Timeline|Timeline Stop)
    (:Update
      (Transformation|SetActorLocationAndRotation (Math|Vector|Lerp(Vector) (Variables|Default|GetNewVar) (.location (Transformation|GetWorldTransform (stale Custom|Move NewParam))) _newtrack_0) (Math|Rotator|Lerp(Rotator) (Variables|Default|GetNewVar_0) (.rotation (Transformation|GetWorldTransform (stale Custom|Move NewParam))) _newtrack_0 true)))))

(event EventBeginPlay
  (bind _asya_qi (Utilities|Casting|CastToYaQi (Variables|1|Get主人)))
  (Variables|Default|SetAs%20Ya%20Qi _asya_qi))

(fn ConstructionScript)

(fn NewFunction0
  (params (角色武器 :type BP%20Sword%20Object%20Reference))
  (bind _skeletal (Variables|BP_Sword_C|GetSkeletal 角色武器))
  (Transformation|DetachFromActor 角色武器 "KeepWorld" "KeepWorld" "KeepWorld")
  (Default|计算特效位置 (.AsBP%20Spawn%20Sword (Utilities|Casting|CastToBP_SpawnSword (Variables|1|Get主人))))
  (Variables|1|Set主人 0)
  (Variables|/Script/Engine.PrimitiveComponent|SetbGenerateOverlapEvents _skeletal false)
  (Collision|SetCollisionEnabled _skeletal "QueryAndPhysics")
  (Physics|SetSimulatePhysics _skeletal true)
  (Physics|AddImpulseatLocation _skeletal (+ (Transformation|GetActorUpVector) 1e+04) (Transformation|GetActorLocation) "pingjie")
  (return))

(fn CheckDamage
  (bind _scene (Variables|Default|GetScene))
  (bind _skeletal (Variables|Default|GetSkeletal))
  (bind _returnvalue (Transformation|GetSocketLocation _skeletal "pingjie"))
  (bind _returnvalue_2 (Transformation|GetWorldLocation _scene))
  (bind (_outhits _returnvalue_3) (Class|KismetSystemLibrary|LineTraceMultiforObjects (Math|Vector|MakeVector (.x _returnvalue_2) (.y _returnvalue_2) -3.124999) (Math|Vector|MakeVector (.x _returnvalue) (.y _returnvalue) -3.124999) (Utilities|Array|MakeArray "ObjectTypeQuery3" "ObjectTypeQuery2") false 0 "ForDuration" true "(R=1.000000,G=0.000000,B=0.000000,A=1.000000)" "(R=0.000000,G=1.000000,B=0.000000,A=1.000000)" 0.1))
  (if _returnvalue_3
    (for _array_element _outhits
      (if (Utilities|DoesObjectImplementInterface (.HitActor (Collision|BreakHitResult _array_element)) "/Game/BP/Character/Enemy/BPI_DamageInterface.BPI_DamageInterface_C")
        (Game|Damage|ApplyDamage (.HitActor (Collision|BreakHitResult _array_element)) (Variables|Default|GetBase%20Damage) 0 0)))))

(fn MoveForward
  (Transformation|AddActorWorldOffset (* (Transformation|GetActorRightVector) (* (Variables|/Game/YaQi/Bp/YaQi.YaQi_C|Get旋转速度 (Variables|Default|GetAs%20Ya%20Qi)) -1e+01))))